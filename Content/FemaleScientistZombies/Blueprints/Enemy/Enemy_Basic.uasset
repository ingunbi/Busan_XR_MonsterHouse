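; Basic enemy character that wanders the navmesh and chases and attacks the player when AI perception senses them.
; Wandering scales speed by hop distance, while chasing focuses on the player and loops an attack montage on arrival.
; AttackCollisionActive/Disactive events gate a per-tick socket-to-socket sphere trace, with a DoOnce limiting each swing to one camera shake and player message.
; Tick also eases yaw toward the player during the attack's opening phase.
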(event `Ai Move Again`
  (bind _returnvalue (`self.K2_GetActorLocation`))
  ;[1 1 1] Ai Perception 범위 안에 들어왔는지에 대한 분기     (T: 범위 내, F: 범위 외)
  (if (stale `self.AIPerception.OnTargetPerceptionUpdated` _output_get) :!label _label
    ;[1 1 1] Focus 설정
    (`AIController.K2_SetFocus` (`AIBlueprintHelperLibrary.GetAIController` self) (`GameplayStatics.GetPlayerPawn` 0))
    (set `CharacterMovementComponent.MaxWalkSpeed` (`self.Attack_Speed`) (`self.CharacterMovement`))
    ;[1 1 1] 범위 내에 있을 때 플레이어를 향하여 이동
    (`|AIMoveTo` self (0.0 0.0 0.0) (`GameplayStatics.GetPlayerPawn` 0) 75.0 :!label _label_2
      (:`OnSuccess`
        (if (`self.Stimulus Successfully Sensed`)
          ;[1 1 1] 플레이어에게 이동 후 공격 애니메이션 재생
          (bind _returnvalue_2 (`self.PlayAnimMontage` (`self.Attack_Anim`) (`self.Attack_Anim_Rate`)))
          (set `self.attacking?` true)
          (bind _returnvalue_3 (* _returnvalue_2 0.3))
          (`KismetSystemLibrary.Delay` _returnvalue_3)
          (set `self.attacking?` false)
          (`KismetSystemLibrary.Delay` _returnvalue_3)
          (`|ExecutionSequence`
            (:`then_0`
              (`self.Attack Reactive`))
            (:`then_1`
              (`KismetSystemLibrary.Delay` _returnvalue_3)
              (goto _label_2)))))
      (:`OnFail`
        ;[1 1 1] 랜덤 위치로 이동
        (`|AIMoveTo` self (stale _output_get) null 1.0 :!label _label_3
          (:`OnSuccess`
            (`KismetSystemLibrary.Delay` (`KismetMathLibrary.RandomFloatInRange` 0.2 1.0))
            (`self.Ai Move Again`))
          (:`OnFail`
            ;[1 1 1] 랜덤으로 이동할 위치 설정
            (bind _randomlocation (`NavigationSystemV1.K2_GetRandomLocationInNavigableRadius` _returnvalue 400.0 null null :!label _label_4))
            (bind _output_get (set `self.Random Location` _randomlocation))
            ;[1 1 1] 이동 거리에 따른 이동 속도 설정
            (if (< (`KismetMathLibrary.Vector_Distance2D` _returnvalue _output_get) 150.0)
              (set `CharacterMovementComponent.MaxWalkSpeed` (`self.Default_Speed_Near`) (`self.CharacterMovement`))
              (goto _label_3)
              (else
                (set `CharacterMovementComponent.MaxWalkSpeed` (`self.Default_Speed_Far`) (`self.CharacterMovement`))
                (goto _label_3)))))))
    (else
      (`AIController.K2_SetFocus` (`AIBlueprintHelperLibrary.GetAIController` self) null)
      (`KismetSystemLibrary.Delay` 3.0)
      (goto _label_4))))

(event `self.AIPerception.OnTargetPerceptionUpdated`
  (params (Actor :type "Actor Object Reference") (Stimulus :type "AIStimulus Structure"))
  ;[1 1 1] Ai Perception 범위 안에 들어왔는지에 대한 분기     (T: 범위 내, F: 범위 외)
  (if (== Actor (`GameplayStatics.GetPlayerPawn` 0))
    (bind _output_get (set `self.Stimulus Successfully Sensed` Stimulus_bSuccessfullySensed))
    (goto _label)))

(event `self.ReceiveBeginPlay`
  ;[1 1 1] 랜덤으로 이동할 위치 설정
  (goto _label_4))

(event `AttackCollisionActive`
  (set `self.attack Motion?` true))

(event `AttackCollisionDisactive`
  (set `self.attack Motion?` false))

(event `self.ReceiveTick`
  (params (DeltaSeconds :type "Float (single-precision)"))
  (bind (_returnvalue_roll _returnvalue_pitch _returnvalue_yaw) (`KismetMathLibrary.BreakRotator` (`KismetMathLibrary.RLerp` (`self.K2_GetActorRotation`) (`KismetMathLibrary.FindLookAtRotation` (`self.K2_GetActorLocation`) (`self.K2_GetActorLocation` (`GameplayStatics.GetPlayerCharacter` 0))) 0.05 true)))
  (`|ExecutionSequence`
    (:`then_0`
      (if (`self.attack Motion?`)
        ;[1 1 1] 애니메이션 동작 중 특정 프레임에 Sphere Trace 발생
        (bind (_outhit _returnvalue) (`KismetSystemLibrary.SphereTraceSingle` :`Start` (`SceneComponent.GetSocketLocation` (`self.Mesh`) (`self.Trace_Start_Socket`)) :`End` (`SceneComponent.GetSocketLocation` (`self.Mesh`) (`self.Trace_End_Socket`)) :`Radius` 10.0 :`TraceChannel` "TraceTypeQuery3" :`DrawDebugType` "ForDuration" :`DrawTime` 1.0))
        (if _returnvalue
          _
          (else
            _))
        (if (== (`.HitActor` (`GameplayStatics.BreakHitResult` _outhit)) (`GameplayStatics.GetPlayerPawn` 0))
          (`/Engine/EditorBlueprintResources/StandardMacros.DoOnce` false :!label _label_5
            (:`Completed`
              (`KismetSystemLibrary.PrintString` "Damaged!")
              (`LegacyCameraShake.StartLegacyCameraShake` (`GameplayStatics.GetPlayerCameraManager` 0) "/Game/Enemy/Resarcher/Blueprint/CS_Resarcher.CS_Resarcher_C")
              (message `/Game/Enemy/damage_recive.resent` (`GameplayStatics.GetPlayerPawn` 0)))))))
    (:`then_1`
      (if (`self.attacking?`)
        (`self.K2_SetActorRotation` (`KismetMathLibrary.MakeRotator` 0.0 0.0 _returnvalue_yaw))))))

(event `Attack Reactive`
  ;[1 1 1] 애니메이션 동작 중 특정 프레임에 Sphere Trace 발생
  (goto _label_5 :!via `Reset`))

(fn `UserConstructionScript`)